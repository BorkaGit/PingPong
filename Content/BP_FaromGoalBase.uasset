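; BP_FaromGoalBase is a base goal Blueprint that shows a player's score on the HUD when a goal occurs.
; OnGoal runs its logic only without authority, so the server, including a listen-server host, skips this HUD update.
; It casts player controller 0's HUD to BP_FaromHUD and passes Score to the first or second player's update on UIRef, chosen by IsFirstPlayer.
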(event EventBeginPlay)

(event Collision|EventActorBeginOverlap
  (params (OtherActor :type Actor%20Object%20Reference)))

(event EventTick
  (params (DeltaSeconds :type Float%20%28single-precision%29)))

(event EventOnGoal
  (bind _score (Variables|Default|GetScore))
  (if (not (Ability|HasAuthority))
    (bind _asbp_farom_hud (Utilities|Casting|CastToBP_FaromHUD (HUD|GetHUD (Game|GetPlayerController 0))))
    (if (Variables|Default|GetbIsFirstPlayer)
      (Default|UpdateFirstPlayerScore (Variables|/Game/BP_FaromHUD.BP_FaromHUD_C|GetUI_Ref _asbp_farom_hud) _score)
      (else
        (Default|UpdateSecondPlayerScore (Variables|/Game/BP_FaromHUD.BP_FaromHUD_C|GetUI_Ref _asbp_farom_hud) _score)))))

(fn ConstructionScript)